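; KeylessDoor is a parametric door that swings on its hinge when the player interacts, with no key check.
; The construction script sizes the panel, optionally builds a three-piece instanced frame, and spaces instanced hinge meshes evenly along its height.
; Interaction scales the OpenTheDoor timeline to the configured duration, then plays or reverses it based on IsOpen, driving hinge yaw toward the configured angle.
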(event `/Game/Blueprints/Interface/IPlayerCanLookAtAndInteractWith.PlayerWantsToInteract`
  (params (PlayerCharacter :type "/Game/Blueprints/PlayerAndGame/PlayerCharacter Object Reference"))
  (`TimelineComponent.SetPlayRate` (`self.Open The Door`) (/ (`TimelineComponent.GetTimelineLength` (`self.Open The Door`)) (`self.How long does it take to open?`)))
  (if (`self.IsOpen`)
    (bind (_direction _percent) (`Timeline|Open The Door` :!label _label)
      (:`Update`
        (`SceneComponent.K2_SetRelativeRotation` (`self.Hinge`) (`KismetMathLibrary.MakeRotator` 0.0 0.0 (* _percent (`self.How many degees to open`) -1.0)) false false)))
    (else
      (goto _label :!via `Reverse`))))

(event `self.ReceiveBeginPlay`
  (goto _label :!via `SetNewTime`))

(fn `PositionOfHinge`
  (params (`Hinge Number` :type Integer))
  (returns (`Position of Hinge` :type "Vector Structure"))
  (locals (BufferCM :type "Float (double-precision)" :default 10.0))
  (bind _returnvalue (* (`self.Hinge Height`) 100.0))
  (bind (_relativescale3d_x _relativescale3d_y _relativescale3d_z) (`KismetMathLibrary.BreakVector` (`SceneComponent.RelativeScale3D` (`self.Mesh-Door`))))
  (return (`KismetMathLibrary.MakeVector` 0.0 0.0 (+ _returnvalue (* `Hinge Number` (/ (- (* _relativescale3d_z 100.0) (* _returnvalue 2.0)) (`KismetMathLibrary.Conv_IntToDouble` (- (`self.Number of Hinges`) 1))))))))

(fn `UserConstructionScript`
  (locals (DoorSize :type "Vector Structure" :default (0.0 0.0 0.0)))
  (bind _hinge_radius (`self.Hinge Radius`))
  (bind _thicc (`self.Thicc`))
  (bind _returnvalue (`KismetMathLibrary.MakeVector` (`self.Wide`) (`self.Thicc`) (`self.Tall`)))
  (bind _returnvalue_2 (* (`self.Thicc`) (`self.FrameThickMult`)))
  (bind _returnvalue_3 (* _thicc (`self.FrameThickMult`)))
  (bind _returnvalue_4 (* (`self.Tall`) (`self.FrameHeightMult`)))
  (bind _returnvalue_5 (`KismetMathLibrary.MakeTransform` (`KismetMathLibrary.MakeVector` (- (* _returnvalue_3 -50.0) (`self.FrameGap`)) (* _thicc 50.0) (* _returnvalue_4 50.0)) (struct) (`KismetMathLibrary.MakeVector` _returnvalue_3 _returnvalue_3 _returnvalue_4)))
  ;[1 1 1] Make Door
  (bind _output_get (set `local.DoorSize` _returnvalue))
  (`SceneComponent.K2_SetRelativeTransform` (`self.Mesh-Door`) (`KismetMathLibrary.MakeTransform` (* _output_get 50.0) (struct) _returnvalue) false true)
  (if (`self.Render door frame`)
    ;[1 1 1] Build door frame
    (`InstancedStaticMeshComponent.AddInstance` (`self.Mesh-Frame`) _returnvalue_5)
    (`InstancedStaticMeshComponent.AddInstance` (`self.Mesh-Frame`) (`KismetMathLibrary.MakeTransform` (`KismetMathLibrary.MakeVector` (+ (* (`self.Wide`) 100.0) (* (`self.Thicc`) (`self.FrameThickMult`) 50.0) (`self.FrameGap`)) (.y (.location _returnvalue_5)) (.z (.location _returnvalue_5))) (struct) (.scale _returnvalue_5)))
    (`InstancedStaticMeshComponent.AddInstance` (`self.Mesh-Frame`) (`KismetMathLibrary.MakeTransform` (`KismetMathLibrary.MakeVector` (* (`self.Wide`) 50.0) (* (`self.Thicc`) 50.0) (+ (* (`self.Tall`) 100.0) (* _returnvalue_2 50.0) (`self.FrameGap`))) (struct) (`KismetMathLibrary.MakeVector` (* (`self.Wide`) 1.5) _returnvalue_2 _returnvalue_2))))
  ;[1 1 1] Make Hinges
  (for _index (range (`self.Number of Hinges`))
    (bind _position_of_hinge (`self.PositionOfHinge` _index))
    (`InstancedStaticMeshComponent.AddInstance` (`self.Mesh-Hinge`) (`KismetMathLibrary.MakeTransform` _position_of_hinge (struct) (`KismetMathLibrary.MakeVector` _hinge_radius _hinge_radius (`self.Hinge Height`))))))