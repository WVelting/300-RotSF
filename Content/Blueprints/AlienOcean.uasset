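; AlienOcean is a construction-script actor that builds an alien ocean surface sized by Width and Height, with no runtime logic.
; The construction script fills a grid centered on the actor with instanced water meshes, spaced 10,000 units apart.
; MakePlanes adds four scaled plane instances around the grid, offset in a pinwheel layout to form a surrounding border of BorderWidth thickness.
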(fn `MakePlanes`
  (bind _border_width (`self.border width`))
  (bind _border_width_2 (`self.border width`))
  (bind _border_width_3 (`self.border width`))
  (bind _border_width_4 (`self.border width`))
  (bind _returnvalue (* _border_width_4 5000.0))
  (bind _returnvalue_2 (* _border_width 5000.0))
  (bind _returnvalue_3 (* _border_width_2 5000.0))
  (bind _returnvalue_4 (* _border_width_3 5000.0))
  (`InstancedStaticMeshComponent.AddInstance` (`self.Planes`) (`KismetMathLibrary.MakeTransform` (`KismetMathLibrary.MakeVector` _returnvalue_3 (+ (* (/ (`KismetMathLibrary.Conv_IntToDouble` (`self.width`)) 2.0) 10000.0) _returnvalue_3)) (struct) (`KismetMathLibrary.MakeVector` (* (+ _border_width_2 (`KismetMathLibrary.Conv_IntToDouble` (`self.height`))) 100.0) (* _border_width_2 100.0) 1.0)))
  (`InstancedStaticMeshComponent.AddInstance` (`self.Planes`) (`KismetMathLibrary.MakeTransform` (`KismetMathLibrary.MakeVector` (* _returnvalue -1.0) (* (+ (* (/ (`KismetMathLibrary.Conv_IntToDouble` (`self.width`)) 2.0) 10000.0) _returnvalue) -1.0)) (struct) (`KismetMathLibrary.MakeVector` (* (+ _border_width_4 (`KismetMathLibrary.Conv_IntToDouble` (`self.height`))) 100.0) (* _border_width_4 100.0) 1.0)))
  (`InstancedStaticMeshComponent.AddInstance` (`self.Planes`) (`KismetMathLibrary.MakeTransform` (`KismetMathLibrary.MakeVector` (+ (* (/ (`KismetMathLibrary.Conv_IntToDouble` (`self.height`)) 2.0) 10000.0) _returnvalue_4) (* _returnvalue_4 -1.0)) (struct) (`KismetMathLibrary.MakeVector` (* _border_width_3 100.0) (* (+ _border_width_3 (`KismetMathLibrary.Conv_IntToDouble` (`self.width`))) 100.0) 1.0)))
  (`InstancedStaticMeshComponent.AddInstance` (`self.Planes`) (`KismetMathLibrary.MakeTransform` (`KismetMathLibrary.MakeVector` (* (+ (* (/ (`KismetMathLibrary.Conv_IntToDouble` (`self.height`)) 2.0) 10000.0) _returnvalue_2) -1.0) _returnvalue_2) (struct) (`KismetMathLibrary.MakeVector` (* _border_width 100.0) (* (+ _border_width (`KismetMathLibrary.Conv_IntToDouble` (`self.width`))) 100.0) 1.0))))

(fn `UserConstructionScript`
  (locals (offsetX :type "Float (double-precision)") (offsetY :type "Float (double-precision)"))
  (set `local.offsetX` (- (/ (`KismetMathLibrary.Conv_IntToDouble` (`self.width`)) 2.0) 0.5))
  (set `local.offsetY` (- (/ (`KismetMathLibrary.Conv_IntToDouble` (`self.height`)) 2.0) 0.5))
  (`self.MakePlanes`)
  (for _index (range (`self.width`))
    (for _index_2 (range (`self.height`))
      (`InstancedStaticMeshComponent.AddInstance` (`self.WaterMESHes`) (`KismetMathLibrary.MakeTransform` (`KismetMathLibrary.MakeVector` (* (- (`KismetMathLibrary.Conv_IntToDouble` _index_2) (`local.offsetY`)) 10000.0) (* (- (`KismetMathLibrary.Conv_IntToDouble` _index) (`local.offsetX`)) 10000.0)))))))